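; BP_Personaje is a 2D player character that handles horizontal movement and jumping through Enhanced Input.
; On BeginPlay it adds the MP_RH mapping context to its player controller's input subsystem.
; IA_Movimiento shifts the actor along local X by the input value times VelocidadMovimiento, without sweep or delta-time scaling, bypassing character movement, while IA_Saltar calls the built-in Jump.
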(event `self.ReceiveBeginPlay`
  (bind _asplayer_controller (cast `PlayerController` (`self.GetController`)))
  (`EnhancedInputSubsystemInterface.AddMappingContext` (pcsubsystem `EnhancedInputLocalPlayerSubsystem` _asplayer_controller) "/Game/2D/InputSystem/MP_RH.MP_RH" 0 (struct)))

(event `EnhancedInput|/Game/2D/InputSystem/IA_Movimiento`
  (params (ActionValue :type "Float (double-precision)") (ElapsedSeconds :type "Float (double-precision)") (TriggeredSeconds :type "Float (double-precision)") (InputAction :type "InputAction Object Reference" :default "/Game/2D/InputSystem/IA_Movimiento.IA_Movimiento"))
  (:`Triggered`
    (`self.K2_AddActorLocalOffset` (`KismetMathLibrary.MakeVector` (* ActionValue (`self.VelocidadMovimiento`))))))

(event `EnhancedInput|/Game/2D/InputSystem/IA_Saltar`
  (params (ActionValue :type "Float (double-precision)") (ElapsedSeconds :type "Float (double-precision)") (TriggeredSeconds :type "Float (double-precision)") (InputAction :type "InputAction Object Reference" :default "/Game/2D/InputSystem/IA_Saltar.IA_Saltar"))
  (:`Triggered`
    (`self.Jump`)))

(fn `UserConstructionScript`)